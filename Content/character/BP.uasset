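; Player character Blueprint handling movement, interaction and the Esc pause menu through Enhanced Input.
; Movement follows fixed world X/Y axes, recording input direction (Yönsellik) and whether movement is held (Hareketdevam).
; Etkileşim sends an interaction message to the first overlapping actor implementing NewInterface; Esc toggles the menu widget, pause, cursor and input mode.
; Kaldıkmı reports being stuck when movement is held but speed is below a threshold.
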(event Input|EnhancedActionEvents|EnhancedInputActionInput_AKSİYON
  (params (ActionValue :type Vector%202D%20Structure) (ElapsedSeconds :type Float%20%28double-precision%29) (TriggeredSeconds :type Float%20%28double-precision%29) (InputAction :type Input%20Action%20Object%20Reference :default "/Game/character/Input/Input_AKSİYON.Input_AKSİYON"))
  (:Triggered
    (Pawn|Input|AddMovementInput "1.000000, 0, 0" (.x ActionValue) false) ; Left/Right
    (Pawn|Input|AddMovementInput "0,-1.000000, 0" (.y ActionValue) false) ; Up/Down
    (Variables|Default|SetYönsellik (Math|Vector2D|MakeVector2D (.x ActionValue) (.y ActionValue))))
  (:Started
    (Variables|Default|Sethareketdevam? true))
  (:Completed
    (Variables|Default|Sethareketdevam? false)))

(event Input|EnhancedActionEvents|EnhancedInputActionEsc_menü
  (params (ActionValue :type Boolean) (ElapsedSeconds :type Float%20%28double-precision%29) (TriggeredSeconds :type Float%20%28double-precision%29) (InputAction :type Input%20Action%20Object%20Reference :default "/Game/character/Input/Esc_menü.Esc_menü"))
  (bind _returnvalue (Game|GetPlayerController 0))
  (:Started
    (if (not (Variables|Default|GetEscmenüsüaçıkmı?))
      (Variables|Default|SetEscmenüsüaçıkmı? true)
      (bind _returnvalue_2 (UserInterface|CreateWidget "/Game/Escmenü_bp.Escmenü_bp_C" _returnvalue))
      (bind _output_get (Variables|Default|SetNewVar_0 _returnvalue_2))
      (UserInterface|Viewport|AddtoViewport _output_get 0)
      (Input|SetInputModeGameandUI _returnvalue (Variables|Default|GetNewVar_0) "DoNotLock" true)
      (Variables|/Script/Engine.PlayerController|SetbShowMouseCursor (Game|GetPlayerController 0) true)
      (Game|SetGamePaused true)
      (else
        (Variables|Default|SetEscmenüsüaçıkmı? false)
        (Widget|RemovefromParent (Variables|Default|GetNewVar_0))
        (Game|SetGamePaused false)
        (Input|SetInputModeGameOnly _returnvalue)
        (Variables|/Script/Engine.PlayerController|SetbShowMouseCursor (Game|GetPlayerController 0) false)))))

(event EventBeginPlay
  (bind _asplayer_controller (Utilities|Casting|CastToPlayerController (Pawn|GetController)))
  (Input|AddMappingContext (PlayerController|LocalPlayerSubsystems|GetEnhancedInputLocalPlayerSubsystem _asplayer_controller) "/Game/character/Input/MAPPING.MAPPING" 0 "(bIgnoreAllPressedKeysUntilRelease=True,bForceImmediately=False)"))

(event Input|ActionEvents|InputActionEtkileşim
  (params (Key :type Key%20Structure :default "None"))
  (:Pressed
    (bind _array_element (Utilities|Array|ForEachLoopwithBreak (Collision|GetOverlappingActors "/Script/Engine.Actor" :!class /Script/Engine.Actor) :!label _label)
      (:LoopBody
        (if (Utilities|DoesObjectImplementInterface _array_element "/Game/NewInterface.NewInterface_C")
          (Class|NewInterface|Etkileşim(Message) _array_element)
          (goto _label Break))))))

(fn ConstructionScript)

(fn Kaldıkmı?
  (return (and (Variables|Default|Gethareketdevam?) (< (Math|Vector|VectorLength (Transformation|GetVelocity)) (Variables|Default|GetKalmanıneşiği)))))